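; Paper2D character Blueprint that switches the sprite's flipbook between attack, fall, run and idle animations.
; UpdateAnimation picks a non-looping flipbook from IsAttacking, then falling state and velocity.
; Space Bar plays the attack and sets IsAttacking through a constant-true branch, so nothing reachable clears it.
; When playback finishes, the sprite switches to the attack flipbook with looping on and restarts if stopped.
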(event OnFinishedPlaying(Sprite)
  (Sprite|SetFlipbook (Variables|Default|GetSprite) "/Game/Sprites/Knight/Attack/FB_Attack.FB_Attack")
  (Components|Timeline|SetLooping (Variables|Default|GetSprite) true)
  (if (not (Audio|Components|Audio|IsPlaying (Variables|Default|GetSprite)))
    (Audio|Components|Audio|Play (Variables|Default|GetSprite))))

(event Custom|UpdateAnimation
  (Sprite|SetFlipbook (Variables|Default|GetSprite) (select (Variables|Default|GetIsAttacking) "/Game/Sprites/Knight/Attack/FB_Attack.FB_Attack" (select (AI|Components|NavMovement|IsFalling (Variables|Character|GetCharacterMovement)) "/Game/Sprites/Knight/JumpAndFall/FB_Fall.FB_Fall" (select (> (Math|Vector|VectorLength (Variables|/Script/Engine.MovementComponent|GetVelocity (Variables|Character|GetCharacterMovement))) 0.0) "/Game/Sprites/Knight/Run/FB_Run.FB_Run" "/Game/Sprites/Knight/Idle/FB_Idle.FB_Idle"))))
  (Components|Timeline|SetLooping (Variables|Default|GetSprite) false))

(event Input|KeyboardEvents|SpaceBar
  (params (Key :type Key%20Structure :default "None"))
  (:Pressed
    (Sprite|SetFlipbook (Variables|Default|GetSprite) "/Game/Sprites/Knight/Attack/FB_Attack.FB_Attack")
    (Components|Timeline|SetLooping (Variables|Default|GetSprite) false)))

(event Input|KeyboardEvents|SpaceBar
  (params (Key :type Key%20Structure :default "None"))
  (:Pressed
    (if true
      (Variables|Default|SetIsAttacking true)
      (else
        (Variables|Default|SetIsAttacking false)))))

(fn ConstructionScript)